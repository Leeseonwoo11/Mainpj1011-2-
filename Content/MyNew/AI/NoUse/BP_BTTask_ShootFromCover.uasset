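; Behavior tree task that makes a TPSEnemy pawn leave its cover state, aim and shoot for a fixed period.
; On execute it switches the enemy's states, starts shooting and sets a one-shot timer that stops fire, restores cover and finishes successfully.
; On abort it stops shooting and clears both aim and cover states, but leaves the timer running.
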(event `self.ReceiveExecuteAI`
  (params (OwnerController :type "AIController Object Reference") (ControlledPawn :type "Pawn Object Reference"))
  (bind _astpsenemy (cast `TPSEnemy` ControlledPawn))
  (bind _output_get (set `self.TPSEnemy` _astpsenemy))
  (`TPSEnemy.SetFalseCoverState` _output_get)
  (`TPSEnemy.SetTrueAimState` _output_get)
  (`TPSEnemy.CStartShooting` _output_get)
  (`KismetSystemLibrary.K2_SetTimerDelegate` (delegate `StopShooting`) 3.0))

(event `self.ReceiveAbortAI`
  (params (OwnerController :type "AIController Object Reference") (ControlledPawn :type "Pawn Object Reference"))
  (bind _tpsenemy (`self.TPSEnemy`))
  (`TPSEnemy.SetFalseCoverState` _tpsenemy)
  (`TPSEnemy.CStopShoothing` _tpsenemy)
  (`TPSEnemy.SetFalseAimState` _tpsenemy)
  (`self.FinishAbort`))

(event `StopShooting`
  (bind _tpsenemy (`self.TPSEnemy`))
  (`TPSEnemy.CStopShoothing` _tpsenemy)
  (`TPSEnemy.SetTrueCoverState` _tpsenemy)
  (`TPSEnemy.SetFalseAimState` _tpsenemy)
  (`self.FinishExecute` true))