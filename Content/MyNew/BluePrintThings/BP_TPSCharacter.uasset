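; Third-person shooter character Blueprint with a hold-to-highlight effect on nearby TPSEnemy actors.
; Holding E scales a Sphere component up to a large radius, and releasing it shrinks the sphere to near zero.
; Sphere overlaps swap each enemy mesh's first material to a vertex-color grid material and restore it on exit.
; The original material is cached in a single NormalMaterial variable shared by all enemies, overwritten on each new overlap.
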(event `self.Sphere.OnComponentBeginOverlap`
  (params (OverlappedComponent :type "PrimitiveComponent Object Reference") (OtherActor :type "Actor Object Reference") (OtherComp :type "PrimitiveComponent Object Reference") (OtherBodyIndex :type Integer) (bFromSweep :type Boolean) (SweepResult :type "HitResult Structure (by ref)"))
  (bind _astpsenemy (cast `TPSEnemy` OtherActor))
  (bind _mesh (`Character.Mesh` _astpsenemy))
  (set `self.NormalMaterial` (`PrimitiveComponent.GetMaterial` _mesh 0))
  (`PrimitiveComponent.SetMaterial` _mesh 0 "/Engine/EditorMaterials/WidgetGridVertexColorMaterial_Ma.WidgetGridVertexColorMaterial_Ma"))

(event `Key|E`
  (params (Key :type "Key Structure"))
  (:`Pressed`
    (`SceneComponent.SetWorldScale3D` (`self.Sphere`) (100.0 100.0 100.0)))
  (:`Released`
    (`SceneComponent.SetWorldScale3D` (`self.Sphere`) (0.1 0.1 0.1))))

(event `self.Sphere.OnComponentEndOverlap`
  (params (OverlappedComponent :type "PrimitiveComponent Object Reference") (OtherActor :type "Actor Object Reference") (OtherComp :type "PrimitiveComponent Object Reference") (OtherBodyIndex :type Integer))
  (bind _astpsenemy (cast `TPSEnemy` OtherActor))
  (`PrimitiveComponent.SetMaterial` (`Character.Mesh` _astpsenemy) 0 (`self.NormalMaterial`)))

(fn `UserConstructionScript`)