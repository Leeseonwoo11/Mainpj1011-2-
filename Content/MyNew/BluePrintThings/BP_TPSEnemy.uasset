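; BP_TPSEnemy is an enemy that shows its health on a bar widget facing the player.
; On BeginPlay it casts the Widget1 component's widget to EnemyHPBar and caches its progress bar.
; Each Tick it sets the bar from StatComp health, assuming a maximum of 100, and rotates the widget toward the player character's mesh rather than the camera.
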(event `self.ReceiveBeginPlay`
  (bind _asenemy_hpbar (cast `/Game/MyNew/HUD/EnemyHPBar` (`WidgetComponent.GetUserWidgetObject` (`self.Widget1`))))
  (set `self.HPProgressbar` (`/Game/MyNew/HUD/EnemyHPBar.ProgressBar_92` _asenemy_hpbar)))

(event `self.ReceiveTick`
  (params (DeltaSeconds :type "Float (single-precision)"))
  (`ProgressBar.SetPercent` (`self.HPProgressbar`) (/ (`TPSEnemyStatComponent.Health` (`self.StatComp`)) 100.0))
  (`SceneComponent.K2_SetWorldRotation` (`self.Widget1`) (`KismetMathLibrary.FindLookAtRotation` (`SceneComponent.K2_GetComponentLocation` (`self.Widget1`)) (`SceneComponent.K2_GetComponentLocation` (`Character.Mesh` (`GameplayStatics.GetPlayerCharacter` 0)))) false false))

(fn `UserConstructionScript`)